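; BP_clientGenerator supplies the cooking game's service counter with a daily queue of villager, hero and merchant clients, one at a time.
; On BeginPlay it spawns one reusable actor per type at a pool point, then randomly picks types with remaining quota, removing exhausted ones and retrying recursively.
; Chosen clients move to the client spawnpoint, with villagers also generating a demand.
; HideClient returns them to the pool, clears the counter widget and selects the next.
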(event `self.ReceiveBeginPlay`
  (bind _returnvalue (`SceneComponent.K2_GetComponentToWorld` (`self.PoolSpawnpoint`)))
  ; Create Pool
  (bind _returnvalue_2 (`|SpawnActorFromClass` "/Game/Blueprints/Cooking/BP_Villager.BP_Villager_C" _returnvalue "Undefined" "MultiplyWithRoot" null self null))
  (set `self.VillagerRef` _returnvalue_2)
  (bind _returnvalue_3 (`|SpawnActorFromClass` "/Game/Blueprints/Cooking/BP_Hero.BP_Hero_C" _returnvalue "Undefined" "MultiplyWithRoot" null self null))
  (set `self.HeroRef` _returnvalue_3)
  (bind _returnvalue_4 (`|SpawnActorFromClass` "/Game/Blueprints/Cooking/BP_Merchant.BP_Merchant_C" _returnvalue "Undefined" "MultiplyWithRoot" null self null))
  (set `self.MerchantRef` _returnvalue_4)
  (`self.SelectNextClient`))

(event `SelectNextClient`
  (bind _dailymerchantquantity (`self.DailyMerchantQuantity`))
  (bind _villagerref (`self.VillagerRef`))
  (bind _dailyclientquantity (`self.DailyClientQuantity`))
  (bind _dailyheroquantity (`self.DailyHeroQuantity`))
  ; Select and show next Client
  (if (and (<= (`self.DailyMerchantQuantity`) 0) (<= (`self.DailyHeroQuantity`) 0) (<= (`self.DailyClientQuantity`) 0))
    (`KismetSystemLibrary.PrintString` "No one left")
    (else
      (switch `/Game/Blueprints/System/E_ClientType` (`KismetArrayLibrary.Array_Random` (`self.ClientType`))
        (:`NewEnumerator0`
          (if (> _dailyclientquantity 0)
            (`/Engine/EditorBlueprintResources/StandardMacros.DecrementInt` _dailyclientquantity
              (:`  `
                (set `self.CurrentClient` _villagerref)
                (`/Game/Blueprints/Cooking/BP_Villager.GenerateDemand` _villagerref)
                (`self.ShowClient` :!label _label)))
            (else
              (`KismetArrayLibrary.Array_RemoveItem` (`self.ClientType`) "NewEnumerator0")
              (`self.SelectNextClient` :!label _label_2))))
        (:`NewEnumerator1`
          (if (> _dailyheroquantity 0)
            (`/Engine/EditorBlueprintResources/StandardMacros.DecrementInt` _dailyheroquantity
              (:`  `
                (set `self.CurrentClient` (`self.HeroRef`))
                (goto _label)))
            (else
              (`KismetArrayLibrary.Array_RemoveItem` (`self.ClientType`) "NewEnumerator1")
              (goto _label_2))))
        (:`NewEnumerator2`
          (if (> _dailymerchantquantity 0)
            (`/Engine/EditorBlueprintResources/StandardMacros.DecrementInt` _dailymerchantquantity
              (:`  `
                (set `self.CurrentClient` (`self.MerchantRef`))
                (goto _label)))
            (else
              (`KismetArrayLibrary.Array_RemoveItem` (`self.ClientType`) "NewEnumerator2")
              (goto _label_2))))))))

(event `ShowClient`
  (bind _currentclient (`self.CurrentClient`))
  (`self.K2_SetActorTransform` _currentclient (`SceneComponent.K2_GetComponentToWorld` (`self.ClientSpawnpoint`)) false false)
  (`/Game/Blueprints/Cooking/BP_client.NotifyPresence` _currentclient))

(event `HideClient`
  (`self.K2_SetActorLocation` (`self.CurrentClient`) (`SceneComponent.K2_GetComponentLocation` (`self.PoolSpawnpoint`)) false false)
  (`Widget.RemoveFromParent` (`/Game/Blueprints/Cooking/BP_ServiceStation.ServiceStationWidgteRef` (`self.ServiceCounterRef`)))
  (set `self.CurrentClient` null)
  (`self.SelectNextClient`))

(fn `UserConstructionScript`)