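; BP_ServiceStation is a cooking-game station where meals are placed to be served.
; SetStation creates a WBP_ServiceStation widget linked to the station and sets it as the cookery pawn's current station widget.
; A MealDetection overlap component stores the overlapping BP_meal as MealToServe and clears it when a meal leaves.
; ClientPresent only prints a debug message announcing a new client.
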(event `self.ReceiveBeginPlay`
  (bind _asbp_cookery_pawn (cast `/Game/Blueprints/Character/Kitchen/BP_CookeryPawn` (`GameplayStatics.GetPlayerPawn` 0)))
  (set `self.Cookery Pawn Ref` _asbp_cookery_pawn))

(event `/Game/Blueprints/System/BPI_Stations.SetStation`
  (bind _returnvalue (`|CreateWidget` "/Game/Blueprints/UI/WBP_ServiceStation.WBP_ServiceStation_C" null self))
  (bind _output_get (set `self.ServiceStationWidgteRef` _returnvalue))
  (set `/Game/Blueprints/Character/Kitchen/BP_CookeryPawn.CurrentStationWidget` _output_get (`self.Cookery Pawn Ref`)))

(event `ClientPresent`
  (`KismetSystemLibrary.PrintString` "new client"))

(event `self.MealDetection.OnComponentBeginOverlap`
  (params (OverlappedComponent :type "PrimitiveComponent Object Reference") (OtherActor :type "Actor Object Reference") (OtherComp :type "PrimitiveComponent Object Reference") (OtherBodyIndex :type Integer) (bFromSweep :type Boolean) (SweepResult :type "HitResult Structure (by ref)"))
  (bind _asbp_meal (cast `/Game/Blueprints/Cooking/Meal/BP_meal` OtherActor))
  (set `self.MealToServe` _asbp_meal)
  (`KismetSystemLibrary.PrintString` "Meal Present"))

(event `self.MealDetection.OnComponentEndOverlap`
  (params (OverlappedComponent :type "PrimitiveComponent Object Reference") (OtherActor :type "Actor Object Reference") (OtherComp :type "PrimitiveComponent Object Reference") (OtherBodyIndex :type Integer))
  (cast `/Game/Blueprints/Cooking/Meal/BP_meal` OtherActor)
  (set `self.MealToServe` null))

(fn `UserConstructionScript`)