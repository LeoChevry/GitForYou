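; Kitchen counter for the cooking game that turns ingredients placed in its pot into a meal.
; Overlaps track ingredients, and each new one updates the cook button, shown for two or three items.
; StartRecipe sums their properties and food types, then SearchMeal filters DTMeal by type through a gate and picks the nearest property vector by squared distance.
; It then destroys the ingredients and spawns BP_meal with that row.
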(event `self.ReceiveBeginPlay`
  (bind _asbp_cookery_pawn (cast `/Game/Blueprints/Character/Cookery/BP_CookeryPawn` (`GameplayStatics.GetPlayerPawn` 0)))
  (set `self.Cookery Pawn Ref` _asbp_cookery_pawn))

(event `self.ReceiveTick`
  (params (DeltaSeconds :type "Float (single-precision)"))
  (for _array_element (`self.IngredientsInPot`)
    (`KismetSystemLibrary.PrintString` (`KismetSystemLibrary.GetDisplayName` _array_element) true true (struct :`G` 0.66 :`B` 1.0 :`A` 1.0) 0.0)))

(event `self.IngredientDetection.OnComponentBeginOverlap`
  (params (OverlappedComponent :type "PrimitiveComponent Object Reference") (OtherActor :type "Actor Object Reference") (OtherComp :type "PrimitiveComponent Object Reference") (OtherBodyIndex :type Integer) (bFromSweep :type Boolean) (SweepResult :type "HitResult Structure (by ref)"))
  (bind _cookinventoryref (`self.CookInventoryRef`))
  (bind _asbp_ingredient (cast `/Game/Blueprints/Cooking/Ingredients/BP_Ingredient` OtherActor))
  (`KismetArrayLibrary.Array_Add` (`self.IngredientsInPot`) _asbp_ingredient)
  (bind _aswbp_cook_inventory (cast `/Game/Blueprints/UI/WBP_CookingStation` (`/Game/Blueprints/Character/Cookery/BP_CookeryPawn.CurrentStationWidget` (`self.Cookery Pawn Ref`))))
  (set `self.CookInventoryRef` _aswbp_cook_inventory)
  (set `/Game/Blueprints/UI/WBP_CookButton.KitchenCounterRef` self (`/Game/Blueprints/UI/WBP_CookingStation.WBP_CookButton` _aswbp_cook_inventory))
  (if (`KismetMathLibrary.InRange_IntInt` (`KismetArrayLibrary.Array_Length` (`self.IngredientsInPot`)) 2 3)
    (`/Game/Blueprints/UI/WBP_CookingStation.VisibilityCookButton` _cookinventoryref "Visible")
    (else
      (`/Game/Blueprints/UI/WBP_CookingStation.VisibilityCookButton` _cookinventoryref "Hidden"))))

(event `self.IngredientDetection.OnComponentEndOverlap`
  (params (OverlappedComponent :type "PrimitiveComponent Object Reference") (OtherActor :type "Actor Object Reference") (OtherComp :type "PrimitiveComponent Object Reference") (OtherBodyIndex :type Integer))
  (bind _ingredientsinpot (`self.IngredientsInPot`))
  (bind _asbp_ingredient (cast `/Game/Blueprints/Cooking/Ingredients/BP_Ingredient` OtherActor))
  (`KismetArrayLibrary.Array_Remove` _ingredientsinpot (`KismetArrayLibrary.Array_Find` _ingredientsinpot _asbp_ingredient)))

(event `StartRecipe`
  (set `self.ShortestDistance` 999.0)
  (set `self.SelectedRow` (struct))
  (set `self.TotalPropreties` (0.0 0.0 0.0))
  (`KismetArrayLibrary.Array_Clear` (`self.CurrentMealTypes`))
  (bind (_arrayindex _arrayelement) (`/Engine/EditorBlueprintResources/StandardMacros.ReverseForEachLoop` (`self.IngredientsInPot`))
    (:`LoopBody`
      (bind _ingredientdata (`/Game/Blueprints/Cooking/Ingredients/BP_Ingredient.IngredientData` _arrayelement))
      (set `self.TotalPropreties` (+ (`/Game/Blueprints/System/PDA_Ingredient.Propreties` _ingredientdata) (`self.TotalPropreties`)))
      (`KismetArrayLibrary.Array_AddUnique` (`self.CurrentMealTypes`) (`/Game/Blueprints/System/PDA_Ingredient.FoodType` _ingredientdata)))
    (:`Completed`
      (`self.SearchMeal`))))

(event `SearchMeal`
  (bind _dt_meal (`self.DT_Meal`))
  (bind _ingredientsinpot (`self.IngredientsInPot`))
  (bind _outrownames (`DataTableFunctionLibrary.GetDataTableRowNames` _dt_meal))
  (for _array_element _outrownames
    (bind _returnvalue (`|GetDataTableRow` _dt_meal _array_element)
      (:`then`
        (bind ((`TargetPropreties_26_0C5B449941A9983D1B5E05AFC70C09BD` _targetpropreties) (`TargetTypes_23_A262167E4D0A158E107C18B279C63B39` _targettypes)) (break `/Game/Blueprints/System/F_Meal` _returnvalue))
        (for _array_element_2 _targettypes
          (if (not (`KismetArrayLibrary.Array_Contains` (`self.CurrentMealTypes`) _array_element_2))
            (goto _label :!via `Close`)))
        (`/Engine/EditorBlueprintResources/StandardMacros.Gate` false :!label _label
          (:`Exit`
            (bind _returnvalue_2 (`KismetMathLibrary.Vector_DistanceSquared` (`self.TotalPropreties`) _targetpropreties))
            (if (< _returnvalue_2 (`self.ShortestDistance`))
              (set `self.ShortestDistance` _returnvalue_2)
              (set `self.SelectedRow` _returnvalue)))))))
  (bind (_arrayindex _arrayelement) (`/Engine/EditorBlueprintResources/StandardMacros.ReverseForEachLoop` _ingredientsinpot)
    (:`LoopBody`
      (`self.K2_DestroyActor` _arrayelement))
    (:`Completed`
      (`KismetArrayLibrary.Array_Clear` _ingredientsinpot)
      (`|SpawnActorFromClass` "/Game/Blueprints/Cooking/Meal/BP_meal.BP_meal_C" (`SceneComponent.K2_GetComponentToWorld` (`self.MealSpawnpoint`)) "Undefined" "MultiplyWithRoot" null (`self.SelectedRow`) null))))

(fn `UserConstructionScript`)