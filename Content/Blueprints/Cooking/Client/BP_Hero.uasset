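; BP_Hero is a hero client in the cooking game, with a hero type, its own look and a reputation reward for the player.
; It picks a stat entry from PossibleHeroStat by index or at random, caches its type and prints its name.
; That entry supplies the body and face materials for the client meshes.
; GetReputation converts Satisfaction into reputation and adds it to the player pawn under that hero type.
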(event `SetCustomHeroStat`
  (params (HeroIndex :type Integer))
  (bind (_name _herotype _herobodymaterial _herofacematerial) (break `/Game/Blueprints/System/F_Hero` (`self.CurrentHeroStat`)))
  (set `self.CurrentHeroStat` (`|GetArrayItem` (`self.PossibleHeroStat`) HeroIndex))
  (set `self.HeroType` _herotype :!label _label)
  (`KismetSystemLibrary.PrintString` (`KismetTextLibrary.Conv_TextToString` _name)))

(event `GenerateHeroStat`
  (set `self.CurrentHeroStat` (`KismetArrayLibrary.Array_Random` (`self.PossibleHeroStat`)))
  (goto _label))

(event `self.SetClientAppearance`
  (params (BodyImages :type "Array of MaterialInstance Object Reference (by ref)") (FaceImages :type "Array of MaterialInstance Object Reference (by ref)"))
  (bind (_name _herotype _herobodymaterial _herofacematerial) (break `/Game/Blueprints/System/F_Hero` (`self.CurrentHeroStat`)))
  (`PrimitiveComponent.SetMaterial` (`self.ClientMesh`) 0 _herobodymaterial)
  (`PrimitiveComponent.SetMaterial` (`self.ClientFaceMesh`) 0 _herofacematerial))

(event `Get Reputation`
  (params (PlayerPawnRef :type "/Game/Blueprints/Character/Kitchen/BP_CookeryPawn Object Reference"))
  (bind _rep (`self.CalculateRep` (`self.Satisfaction`)))
  (`/Game/Blueprints/Character/Kitchen/BP_CookeryPawn.Update Reputation` PlayerPawnRef _rep (`self.HeroType`)))

(fn `UserConstructionScript`
  (`parent.UserConstructionScript`))