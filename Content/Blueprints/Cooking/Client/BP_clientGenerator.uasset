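; BP_clientGenerator feeds clients (villager, hero, merchant) one at a time into the cooking game's service.
; On BeginPlay it spawns one reusable actor of each type at a hidden pool point, then teleports the current one to the client spawn point.
; Selection is either random within daily quotas, re-rolling exhausted types, or a scripted custom sequence.
; Hiding a client returns it to the pool, clears the counter widget and picks the next after a delay.
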(event `self.ReceiveBeginPlay`
  (bind _villagerref (`self.VillagerRef`))
  (bind _heroref (`self.HeroRef`))
  (bind _returnvalue (`SceneComponent.K2_GetComponentToWorld` (`self.PoolSpawnpoint`)))
  ; Create Pool
  (bind _returnvalue_2 (`|SpawnActorFromClass` "/Game/Blueprints/Cooking/Client/BP_Villager.BP_Villager_C" _returnvalue "Undefined" "MultiplyWithRoot" null self null))
  (set `self.VillagerRef` _returnvalue_2)
  (bind _returnvalue_3 (`|SpawnActorFromClass` "/Game/Blueprints/Cooking/Client/BP_Hero.BP_Hero_C" _returnvalue "Undefined" "MultiplyWithRoot" null self null))
  (set `self.HeroRef` _returnvalue_3)
  (bind _returnvalue_4 (`|SpawnActorFromClass` "/Game/Blueprints/Cooking/Client/BP_Merchant.BP_Merchant_C" _returnvalue "Undefined" "MultiplyWithRoot" null self null))
  (set `self.MerchantRef` _returnvalue_4)
  (if (not (`self.RandomClient`))
    (set `self.CustomClients` (`|MakeArray` _heroref _villagerref _heroref _villagerref _villagerref :!type "/Game/Blueprints/Cooking/Client/BP_client Object Reference")))
  (`self.SelectNextClient`))

(event `SelectNextClient`
  (bind _dailymerchantquantity (`self.DailyMerchantQuantity`))
  (bind _villagerref (`self.VillagerRef`))
  (bind _customclientid (`self.CustomClientID`))
  (bind _dailyclientquantity (`self.DailyClientQuantity`))
  (bind _dailyheroquantity (`self.DailyHeroQuantity`))
  (bind _heroref (`self.HeroRef`))
  (bind _output (`|GetArrayItem` (`self.CustomClients`) _customclientid))
  ; Select and show next Client
  (if (`self.RandomClient`)
    (if (and (<= (`self.DailyMerchantQuantity`) 0) (<= (`self.DailyHeroQuantity`) 0) (<= (`self.DailyClientQuantity`) 0))
      (`KismetSystemLibrary.PrintString` "No one left")
      (else
        (switch `/Game/Blueprints/System/E_ClientType` (`KismetArrayLibrary.Array_Random` (`self.ClientType`))
          (:`NewEnumerator0`
            (if (> _dailyclientquantity 0)
              (`/Engine/EditorBlueprintResources/StandardMacros.DecrementInt` _dailyclientquantity
                (:`  `
                  (set `self.CurrentClient` _villagerref)
                  (`/Game/Blueprints/Cooking/Client/BP_Villager.GenerateDemand` _villagerref)
                  (`self.ShowClient` :!label _label)))
              (else
                (`KismetArrayLibrary.Array_RemoveItem` (`self.ClientType`) "NewEnumerator0")
                (`self.SelectNextClient` :!label _label_2))))
          (:`NewEnumerator1`
            (if (> _dailyheroquantity 0)
              (`/Engine/EditorBlueprintResources/StandardMacros.DecrementInt` _dailyheroquantity
                (:`  `
                  (set `self.CurrentClient` _heroref)
                  (`/Game/Blueprints/Cooking/Client/BP_Villager.GenerateDemand` _heroref)
                  (`/Game/Blueprints/Cooking/Client/BP_Hero.GenerateHeroStat` _heroref)
                  (goto _label)))
              (else
                (`KismetArrayLibrary.Array_RemoveItem` (`self.ClientType`) "NewEnumerator1")
                (goto _label_2))))
          (:`NewEnumerator2`
            (if (> _dailymerchantquantity 0)
              (`/Engine/EditorBlueprintResources/StandardMacros.DecrementInt` _dailymerchantquantity
                (:`  `
                  (set `self.CurrentClient` (`self.MerchantRef`))
                  (goto _label)))
              (else
                (`KismetArrayLibrary.Array_RemoveItem` (`self.ClientType`) "NewEnumerator2")
                (goto _label_2)))))))
    (else
      (`/Engine/EditorBlueprintResources/StandardMacros.IsValid` _output
        (:`Is Valid`
          (bind _output_get (set `self.CurrentClient` _output))
          (`/Game/Blueprints/Cooking/Client/BP_Villager.SetCustomDemand` _output_get _customclientid)
          (`self.ShowClient`)
          (`/Engine/EditorBlueprintResources/StandardMacros.IncrementInt` _customclientid))
        (:`Is Not Valid`
          (`KismetSystemLibrary.PrintString` "No client left"))))))

(event `HideClient`
  (`self.K2_SetActorLocation` (`self.CurrentClient`) (`SceneComponent.K2_GetComponentLocation` (`self.PoolSpawnpoint`)) false false)
  (`Widget.RemoveFromParent` (`/Game/Blueprints/Cooking/BP_ServiceStation.ServiceStationWidgteRef` (`self.ServiceCounterRef`)))
  (set `self.CurrentClient` null)
  (`KismetSystemLibrary.Delay` 1.0)
  (`self.SelectNextClient`))

(event `ShowClient`
  (bind _currentclient (`self.CurrentClient`))
  (`self.K2_SetActorTransform` _currentclient (`SceneComponent.K2_GetComponentToWorld` (`self.ClientSpawnpoint`)) false false)
  (`/Game/Blueprints/Cooking/Client/BP_client.NotifyPresence` _currentclient))

(fn `UserConstructionScript`)