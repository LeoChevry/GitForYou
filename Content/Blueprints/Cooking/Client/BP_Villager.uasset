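; BP_Villager is a cooking client that orders a meal at the service counter, then rates and pays for it.
; Demands are randomly generated or loaded from the CustomClients data table, covering ingredient, food type, stat intensity or quantity.
; Talk shows the demand text, or scores the waiting meal, granting half credit for near-miss stats.
; Satisfaction selects a printed reaction and scales gold; BP_Hero instances also award reputation.
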(event `self.SetCustomDemand`
  (params (ClientID :type Integer))
  (bind _returnvalue (`|GetDataTableRow` (`self.CustomClients`) (`KismetStringLibrary.Conv_StringToName` (`KismetStringLibrary.Conv_IntToString` ClientID)))
    (:`then`
      (bind (_demandtypes _ingredienttype _ingredient _stattype _statintensity _ingredientquantityr _demand) (break `/Game/Blueprints/System/F_CustomClient` _returnvalue))
      (set `self.CurrentDemands` _demandtypes)
      (set `self.IngredientTypeDemand` _ingredienttype)
      (set `self.SpecificIngredientDemand` _ingredient)
      (set `self.StatDemand` _stattype)
      (set `self.StatIntensity` _statintensity)
      (set `self.IngredientQuantity` _ingredientquantityr)
      (set `self.FullDemand` _demand))))

(event `GenerateDemand`
  (bind _currentdemands (`self.CurrentDemands`))
  (bind _demandtext (`self.DemandText`))
  ; Generate Demands
  (`self.SetupClient` (`KismetArrayLibrary.Array_Random` (`self.VillagerMaterials`)))
  (`KismetSystemLibrary.DelayUntilNextTick`)
  (set `self.TempDemandTypes` (`self.DemandTypes`))
  (for _ (range (+ (`KismetMathLibrary.RandomInteger` 2) 1))
    (bind _output_get (set `self.TempDemand` (`KismetArrayLibrary.Array_Random` (`self.TempDemandTypes`))))
    (`KismetArrayLibrary.Array_Add` _currentdemands _output_get)
    (`KismetArrayLibrary.Array_RemoveItem` (`self.TempDemandTypes`) (`self.TempDemand`)))
  (for (_array_element _array_index) _currentdemands
    (switch `/Game/Blueprints/System/E_DemandType` _array_element
      (:`NewEnumerator0`
        (bind _output_get_2 (set `self.IngredientTypeDemand` (cast `/Game/Blueprints/System/E_FoodType` (`KismetMathLibrary.Conv_IntToByte` (`KismetMathLibrary.RandomInteger` (- (enumcount `/Game/Blueprints/System/E_FoodType`) 1))))))
        (set `self.DemandText` (`|GenericToText` _output_get_2)))
      (:`NewEnumerator1`
        (bind _output_get_3 (set `self.SpecificIngredientDemand` (`KismetArrayLibrary.Array_Random` (`self.Ingredients`))))
        (set `self.DemandText` (`KismetTextLibrary.Conv_NameToText` (`/Game/Blueprints/System/PDA_Ingredient.Name` _output_get_3))))
      (:`NewEnumerator2`
        (bind _output_get_4 (set `self.StatDemand` (cast `/Game/Blueprints/System/E_IngredientProprety` (`KismetMathLibrary.Conv_IntToByte` (`KismetMathLibrary.RandomInteger` (- (enumcount `/Game/Blueprints/System/E_IngredientProprety`) 1))))))
        (bind _output_get_5 (set `self.StatIntensity` (cast `/Game/Blueprints/System/E_Intensity` (`KismetMathLibrary.Conv_IntToByte` (`KismetMathLibrary.RandomInteger` (- (enumcount `/Game/Blueprints/System/E_Intensity`) 1))))))
        (set `self.DemandText` (`|FormatText` "{Intensity} {StatType}" (`|GenericToText` _output_get_5) (`|GenericToText` _output_get_4))))
      (:`NewEnumerator4`
        (bind _output_get_6 (set `self.IngredientQuantity` (`KismetMathLibrary.RandomIntegerInRange` 2 3)))
        (set `self.DemandText` (`|FormatText` "{Quantity} ingredients" _output_get_6))))
    (switch `int` _array_index
      (:`0`
        (bind _output_get_7 (set `self.Demand1` _demandtext))
        (set `self.FullDemand` _output_get_7))
      (:`1`
        (bind _output_get_8 (set `self.Demand2` _demandtext))
        (set `self.FullDemand` (`|FormatText` "{Demand1} and {Demand2}" _output_get_7 _output_get_8)))
      (:`2`
        (bind _output_get_9 (set `self.Demand3` _demandtext))
        (set `self.FullDemand` (`|FormatText` "{Demand1}, {Demand2} and {Demand3}" _output_get_7 _output_get_8 _output_get_9))))))

(event `self.Talk`
  (bind _value (`BlueprintMapLibrary.Map_Find` (`self.StatIntensityRange`) (`self.StatIntensity`)))
  (bind _value_2 (`BlueprintMapLibrary.Map_Find` (`self.EnlargeStatIntensityRange`) (`self.StatIntensity`)))
  (bind _servicecounterref (`/Game/Blueprints/Cooking/Client/BP_clientGenerator.ServiceCounterRef` (`self.SpawnerRef`)))
  (bind _mealtoserve (`/Game/Blueprints/Cooking/BP_ServiceStation.MealToServe` _servicecounterref))
  (bind _servicestationwidgteref (`/Game/Blueprints/Cooking/BP_ServiceStation.ServiceStationWidgteRef` _servicecounterref))
  (bind _usedingredients (`/Game/Blueprints/Cooking/Meal/BP_meal.UsedIngredients` _mealtoserve))
  (bind (_x _y _z _w) (`KismetMathLibrary.BreakVector4` (`/Game/Blueprints/Cooking/Meal/BP_meal.CurrentStat` _mealtoserve)))
  (bind _array (`|MakeArray` _x _y _z _w))
  ; Set Satisfaction Datas
  (set `self.Satisfaction` 0.0)
  (set `self.SatisfactionIncrement` (/ 100 (`KismetArrayLibrary.Array_Length` (`self.CurrentDemands`))))
  (if (== _mealtoserve null)
    ; Show demand text box
    (`/Engine/EditorBlueprintResources/StandardMacros.IsValid` _servicestationwidgteref
      (:`Is Valid`
        (`/Game/Blueprints/UI/WBP_TalkingBox.UpdateTextBlock` (`/Game/Blueprints/UI/WBP_ServiceStation.WBP_TalkingBox` _servicestationwidgteref) (`self.FullDemand`))
        (`UserWidget.AddToViewport` _servicestationwidgteref 0)))
    (else
      ; Serve Meal & set satisfaction
      (for _array_element (`self.CurrentDemands`)
        (switch `/Game/Blueprints/System/E_DemandType` _array_element
          (:`NewEnumerator0`
            (for _array_element_2 _usedingredients
              (if (`|EnumEquality` (`/Game/Blueprints/System/PDA_Ingredient.FoodType` _array_element_2) (`self.IngredientTypeDemand`))
                (`self.IncrementSatisfaction` (`self.SatisfactionIncrement`))
                (break))))
          (:`NewEnumerator1`
            (if (`KismetArrayLibrary.Array_Contains` _usedingredients (`self.SpecificIngredientDemand`))
              (`self.IncrementSatisfaction` (`self.SatisfactionIncrement`))))
          (:`NewEnumerator2`
            (if (`KismetMathLibrary.InRange_FloatFloat` (`|GetArrayItem` _array (`KismetMathLibrary.Conv_ByteToInt` (`self.StatDemand`))) (`KismetMathLibrary.BreakVector2D` _value) (`.Y` (`KismetMathLibrary.BreakVector2D` _value)) true false)
              (`self.IncrementSatisfaction` (`self.SatisfactionIncrement`))
              (elif (`KismetMathLibrary.InRange_FloatFloat` (`|GetArrayItem` _array (`KismetMathLibrary.Conv_ByteToInt` (`self.StatDemand`))) (`KismetMathLibrary.BreakVector2D` _value_2) (`.Y` (`KismetMathLibrary.BreakVector2D` _value_2)) true false)
                (`self.IncrementSatisfaction` (/ (`self.SatisfactionIncrement`) 2.0)))))
          (:`NewEnumerator4`
            (if (== (`self.IngredientQuantity`) (`KismetArrayLibrary.Array_Length` _usedingredients))
              (`self.IncrementSatisfaction` (`self.SatisfactionIncrement`))))))
      (`self.MealServed`))))

(event `MealServed`
  ; Check satisfaction
  (bind (_keypin _valuepin) (`|MapForEach` (`self.SatisfactionText`) :!label _label)
    (:`then`
      (bind (_x _y) (`KismetMathLibrary.BreakVector2D` _keypin))
      (if (`KismetMathLibrary.InRange_FloatFloat` (`self.Satisfaction`) _x _y true false)
        (`KismetSystemLibrary.PrintString` _valuepin) ; Print satisfaction
        (`self.K2_DestroyActor` (`/Game/Blueprints/Cooking/BP_ServiceStation.MealToServe` (`/Game/Blueprints/Cooking/Client/BP_clientGenerator.ServiceCounterRef` (`self.SpawnerRef`))))
        (`self.Pay`)
        (`KismetArrayLibrary.Array_Clear` (`self.CurrentDemands`))
        (`/Game/Blueprints/Cooking/Client/BP_clientGenerator.HideClient` (`self.SpawnerRef`))
        (goto _label :!via `BreakPin`)))))

(event `Pay`
  (bind _cookery_pawn_ref (`/Game/Blueprints/Cooking/BP_ServiceStation.Cookery Pawn Ref` (`/Game/Blueprints/Cooking/Client/BP_clientGenerator.ServiceCounterRef` (`self.SpawnerRef`))))
  (bind _gold (`self.CalculateGold` (`self.Satisfaction`)))
  (`/Game/Blueprints/Character/Kitchen/BP_CookeryPawn.UpdateGold` _cookery_pawn_ref _gold)
  (bind _asbp_hero (cast `/Game/Blueprints/Cooking/Client/BP_Hero` self))
  (`/Game/Blueprints/Cooking/Client/BP_Hero.Get Reputation` _asbp_hero _cookery_pawn_ref))

(fn `CalculateGold`
  (params (Satisfaction :type "Float (double-precision)"))
  (returns (Gold :type Integer))
  (return (`KismetMathLibrary.Round` (* (/ Satisfaction 100.0) (+ (* (`self.GoldMultiplier`) (* (`self.FurthestBiomeUnlocked`) 10)) (`KismetMathLibrary.RandomIntegerInRange` 1 5))))))

(fn `CalculateRep`
  (params (Satisfaction :type "Float (double-precision)"))
  (returns (Rep :type Integer))
  (return (`KismetMathLibrary.Round` (* (/ Satisfaction 100.0) (+ (`self.FurthestBiomeUnlocked`) (`self.RepBonus`) (`KismetMathLibrary.RandomIntegerInRange` 1 5))))))

(fn `IncrementSatisfaction`
  (params (SatisfactionIncrement :type "Float (double-precision)"))
  (set `self.Satisfaction` (+ (`self.Satisfaction`) SatisfactionIncrement)))

(fn `UserConstructionScript`
  (`parent.UserConstructionScript`))