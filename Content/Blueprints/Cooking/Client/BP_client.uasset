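; BP_client is a customer character in the cooking game, driven through a reference to its spawner.
; On NotifyPresence it tells the spawner's service counter that a client is present and enables talking; Talk asks the spawner to hide the client.
; SetClientAppearance applies random materials from supplied body and face lists to two meshes.
; SetCustomDemand takes a client ID but has no logic here.
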(event `NotifyPresence`
  (`/Game/Blueprints/Cooking/BP_ServiceStation.ClientPresent` (`/Game/Blueprints/Cooking/Client/BP_clientGenerator.ServiceCounterRef` (`self.SpawnerRef`)))
  (set `self.CanTalk` true))

(event `Talk`
  (`/Game/Blueprints/Cooking/Client/BP_clientGenerator.HideClient` (`self.SpawnerRef`)))

(event `SetCustomDemand`
  (params (ClientID :type Integer)))

(event `SetClientAppearance`
  (params (BodyImages :type "Array of MaterialInstance Object Reference") (FaceImages :type "Array of MaterialInstance Object Reference"))
  (`PrimitiveComponent.SetMaterial` (`self.ClientMesh`) 0 (`KismetArrayLibrary.Array_Random` BodyImages))
  (`PrimitiveComponent.SetMaterial` (`self.ClientFaceMesh`) 0 (`KismetArrayLibrary.Array_Random` FaceImages)))

(fn `UserConstructionScript`)