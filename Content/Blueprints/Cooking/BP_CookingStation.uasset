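; Cooking station for the kitchen that takes over the saved dungeon inventory and turns two or three selected ingredients into a meal.
; Its widget handles selection and shows summed stats, then chosen ingredients spawn on the counter, with focus passing along as each enters the pot.
; Once all are in, it spawns the DTMeal row nearest the Vector4 stat total by Euclidean distance, or a fallback row when none is close enough.
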(event `self.ReceiveBeginPlay`
  (set `self.IngredientSpawnPoints` (`|MakeArray` (`self.IngredientSpawnPoint1`) (`self.IngredientSpawnPoint2`) (`self.IngredientSpawnPoint3`))))

(event `/Game/Blueprints/System/BPI_Stations.SetStation`
  (params (KitchenPawnRef :type "/Game/Blueprints/Character/Kitchen/BP_CookeryPawn Object Reference"))
  (bind _kitchen_inventory (`self.Kitchen Inventory`))
  (bind _saveddungeoninventory (`/Game/Blueprints/System/GI_Main.SavedDungeonInventory` (cast `/Game/Blueprints/System/GI_Main` (`GameplayStatics.GetGameInstance`) :!pure true)))
  (set `self.Cookery Pawn Ref` KitchenPawnRef)
  (bind _returnvalue (`|CreateWidget` "/Game/Blueprints/UI/WBP_CookingStation.WBP_CookingStation_C" null self))
  (bind _output_get (set `self.WBP CookingStationRef` _returnvalue))
  (set `/Game/Blueprints/Character/Kitchen/BP_CookeryPawn.CurrentStationWidget` _output_get (`self.Cookery Pawn Ref`))
  (`UserWidget.AddToViewport` _output_get 0)
  ; Transfer dungeon inventory
  (`KismetArrayLibrary.Array_Append` _kitchen_inventory _saveddungeoninventory)
  (`KismetArrayLibrary.Array_Clear` _saveddungeoninventory)
  (`/Game/Blueprints/UI/WBP_CookingStation.UpdateInventory` (`self.WBP CookingStationRef`) _kitchen_inventory)
  (`/Game/Blueprints/UI/WBP_CookingStation.UpdateDemand` (`self.WBP CookingStationRef`) (`/Game/Blueprints/Character/Kitchen/BP_CookeryPawn.CurrentDemand` (`self.Cookery Pawn Ref`))))

(event `/Game/Blueprints/System/BPI_Stations.Interact`
  (`/Game/Blueprints/UI/WBP_CookingStation.ClickPrepare` (`self.WBP CookingStationRef`)))

(event `Select Ingredient`
  (params (IngredientToSelect :type "/Game/Blueprints/System/PDA_Ingredient Object Reference"))
  (bind _wbp_cookingstationref (`self.WBP CookingStationRef`))
  ; item Selection
  (set `self.TotalStats` (+ (`/Game/Blueprints/System/PDA_Ingredient.Stats` IngredientToSelect) (`self.TotalStats`)))
  (`KismetArrayLibrary.Array_Add` (`self.IngredientsToCook`) IngredientToSelect)
  (`/Game/Blueprints/UI/WBP_CookingStation.UpdateSlider` (`self.WBP CookingStationRef`) (`self.TotalStats`) :!label _label)
  (if (`KismetMathLibrary.InRange_IntInt` (`KismetArrayLibrary.Array_Length` (`self.IngredientsToCook`)) 2 3)
    (`/Game/Blueprints/UI/WBP_CookingStation.VisibilityCookButton` _wbp_cookingstationref "Visible")
    (else
      (`/Game/Blueprints/UI/WBP_CookingStation.VisibilityCookButton` _wbp_cookingstationref "Hidden"))))

(event `Deselect Ingredient`
  (params (`Ingredient to deselect` :type "/Game/Blueprints/System/PDA_Ingredient Object Reference"))
  ; item Selection
  (set `self.TotalStats` (- (`self.TotalStats`) (`/Game/Blueprints/System/PDA_Ingredient.Stats` `Ingredient to deselect`)))
  (`KismetArrayLibrary.Array_RemoveItem` (`self.IngredientsToCook`) `Ingredient to deselect`)
  (goto _label))

(event `StartRecipe`
  ; SetUp Ingredients
  (bind (_arrayindex _arrayelement) (`/Engine/EditorBlueprintResources/StandardMacros.ReverseForEachLoop` (`self.IngredientsToCook`))
    (:`LoopBody`
      (`KismetArrayLibrary.Array_Remove` (`self.Kitchen Inventory`) (`KismetArrayLibrary.Array_Find` (`self.Kitchen Inventory`) _arrayelement)))
    (:`Completed`
      (for (_array_element _array_index) (`self.IngredientsToCook`)
        (`KismetArrayLibrary.Array_AddUnique` (`self.CurrentMealTypes`) (`/Game/Blueprints/System/PDA_Ingredient.FoodType` _array_element))
        (bind _returnvalue (`|SpawnActorFromClass` "/Game/Blueprints/Cooking/Ingredients/BP_Ingredient.BP_Ingredient_C" (`SceneComponent.K2_GetComponentToWorld` (`|GetArrayItem` (`self.IngredientSpawnPoints`) _array_index)) "Undefined" "MultiplyWithRoot" null _array_element null))
        (`KismetArrayLibrary.Array_Add` (`self.IngredientOnCounter`) _returnvalue)
        (`/Engine/EditorBlueprintResources/StandardMacros.DoOnce` false :!label _label_2
          (:`Completed`
            (if (`/Game/Blueprints/Character/Kitchen/BP_CookeryController.usingGamepad` (cast `/Game/Blueprints/Character/Kitchen/BP_CookeryController` (`GameplayStatics.GetPlayerController` 0) :!pure true))
              (set `self.FocusedObject` _returnvalue)
              (`/Game/Blueprints/Cooking/Ingredients/BP_Ingredient.SetFocus` _returnvalue true)))))
      (`/Game/Blueprints/UI/WBP_CookingStation.DeselectAllSlots` (`self.WBP CookingStationRef`))
      (goto _label_2 :!via `Reset`))))

(event `self.IngredientDetection.OnComponentBeginOverlap`
  (params (OverlappedComponent :type "PrimitiveComponent Object Reference") (OtherActor :type "Actor Object Reference") (OtherComp :type "PrimitiveComponent Object Reference") (OtherBodyIndex :type Integer) (bFromSweep :type Boolean) (SweepResult :type "HitResult Structure (by ref)"))
  (bind _ingredientoncounter (`self.IngredientOnCounter`))
  (bind _ingredientinpot (`self.IngredientInPot`))
  (bind _ingredientinpot_2 (`self.IngredientInPot`))
  (bind _returnvalue (`KismetArrayLibrary.Array_Length` _ingredientinpot_2))
  (bind _asbp_ingredient (cast `/Game/Blueprints/Cooking/Ingredients/BP_Ingredient` OtherActor))
  (`/Game/Blueprints/Cooking/Ingredients/BP_Ingredient.SetFocus` _asbp_ingredient false)
  (bind _output (`|GetArrayItem` _ingredientoncounter (+ (`KismetArrayLibrary.Array_Find` _ingredientoncounter _asbp_ingredient) 1)))
  (`/Game/Blueprints/Cooking/Ingredients/BP_Ingredient.SetFocus` _output true)
  (set `self.FocusedObject` _output)
  (`KismetArrayLibrary.Array_Add` _ingredientinpot_2 _asbp_ingredient)
  (`KismetSystemLibrary.PrintString` (`KismetStringLibrary.Conv_IntToString` _returnvalue))
  (`KismetSystemLibrary.PrintString` (`KismetStringLibrary.Conv_IntToString` _returnvalue))
  (if (>= _returnvalue (`KismetArrayLibrary.Array_Length` (`self.IngredientsToCook`)))
    (`KismetSystemLibrary.Delay` 1.0)
    (`self.SearchMeal`)
    (bind (_arrayindex _arrayelement) (`/Engine/EditorBlueprintResources/StandardMacros.ReverseForEachLoop` _ingredientinpot)
      (:`LoopBody`
        (`self.K2_DestroyActor` _arrayelement))
      (:`Completed`
        (`KismetArrayLibrary.Array_Clear` _ingredientinpot)))))

(event `SearchMeal`
  (bind _dt_meal (`self.DT_Meal`))
  ; Meal Selection
  (bind _outrownames (`DataTableFunctionLibrary.GetDataTableRowNames` _dt_meal))
  (for _array_element _outrownames :!label _label_3
    (bind _returnvalue (`|GetDataTableRow` _dt_meal _array_element)
      (:`then`
        (bind _distance (`self.CalculateDistVector4` (`self.TotalStats`) (`.TargetPropreties_27_0C5B449941A9983D1B5E05AFC70C09BD` (break `/Game/Blueprints/System/F_Meal` _returnvalue))))
        (if (< _distance (`self.ShortestDistance`))
          (bind _output_get (set `self.ShortestDistance` _distance))
          (set `self.SelectedRow` _returnvalue)
          (if (== _output_get 0.0)
            (`self.Break Search Meal`))))))
  (if (> (`self.ShortestDistance`) 40.0)
    (bind _returnvalue_2 (`|GetDataTableRow` (`self.DT_Meal`) "5")
      (:`then`
        (set `self.SelectedRow` _returnvalue_2))))
  (bind _returnvalue_3 (`|SpawnActorFromClass` "/Game/Blueprints/Cooking/Meal/BP_meal.BP_meal_C" (`SceneComponent.K2_GetComponentToWorld` (`self.MealSpawnpoint`)) "Undefined" "MultiplyWithRoot" null (`self.SelectedRow`) (`self.IngredientsToCook`) null))
  (set `self.FocusedObject` _returnvalue_3)
  (`KismetArrayLibrary.Array_Clear` (`self.IngredientsToCook`))
  (`KismetArrayLibrary.Array_Clear` (`self.IngredientOnCounter`))
  (set `self.ShortestDistance` 9999.0)
  (set `self.SelectedRow` (struct))
  (`KismetArrayLibrary.Array_Clear` (`self.CurrentMealTypes`)))

(event `Break Search Meal`
  ; Meal Selection
  (goto _label_3 :!via `Break`))

(fn `CalculateDistVector4`
  (params (V1 :type "Vector4 Structure") (V2 :type "Vector4 Structure"))
  (returns (Distance :type "Float (double-precision)"))
  (bind (_x _y _z _w) (`KismetMathLibrary.BreakVector4` V2))
  (bind (_x_2 _y_2 _z_2 _w_2) (`KismetMathLibrary.BreakVector4` V1))
  (return (`KismetMathLibrary.Sqrt` (+ (`KismetMathLibrary.Square` (- _x_2 _x)) (`KismetMathLibrary.Square` (- _y_2 _y)) (`KismetMathLibrary.Square` (- _z_2 _z)) (`KismetMathLibrary.Square` (- _w_2 _w))))))

(fn `UserConstructionScript`)