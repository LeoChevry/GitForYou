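; BP_Hero is a hero client in the cooking game that grants the player reputation tied to its hero type.
; GenerateHeroStat picks a random entry from PossibleHeroStat, passes its material to SetupClient, stores the hero type and prints the name.
; GetReputation scales BaseReputation by a reward multiplier and sends it, with that type, to the player pawn's UpdateReputation.
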(event `GenerateHeroStat`
  (bind _output_get (set `self.CurrentHeroStat` (`KismetArrayLibrary.Array_Random` (`self.PossibleHeroStat`))))
  (bind (_name _herotype _heromaterial) (break `/Game/Blueprints/System/F_Hero` _output_get))
  (`self.SetupClient` _heromaterial)
  (set `self.HeroType` _herotype)
  (`KismetSystemLibrary.PrintString` (`KismetTextLibrary.Conv_TextToString` _name)))

(event `Get Reputation`
  (params (`Reward Multiplier` :type "Float (double-precision)") (PlayerPawnRef :type "/Game/Blueprints/Character/Kitchen/BP_CookeryPawn Object Reference"))
  (`/Game/Blueprints/Character/Kitchen/BP_CookeryPawn.Update Reputation` PlayerPawnRef (* (`self.BaseReputation`) `Reward Multiplier`) (`self.HeroType`)))

(fn `UserConstructionScript`
  (`parent.UserConstructionScript`))