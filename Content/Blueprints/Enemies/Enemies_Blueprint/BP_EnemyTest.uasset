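; BP_EnemyTest is a test enemy character that takes damage and is destroyed when its health runs out.
; The construction script reads its name from EnemyStats, and BeginPlay stores the spawn location as a patrol anchor and applies walk speed.
; TakeDamage subtracts health behind a short hit cooldown and prints debug messages, while Tick polls health to destroy the actor.
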(event `self.ReceiveTick`
  (params (DeltaSeconds :type "Float (single-precision)"))
  (if (<= (`self.Health`) 0)
    (`self.K2_DestroyActor`)))

(event `self.ReceiveBeginPlay`
  ; Set le point de patrouille de base
  (set `self.Anchor` (`self.K2_GetActorLocation`))
  (set `CharacterMovementComponent.MaxWalkSpeed` (`self.WalkSpeed`) (`self.CharacterMovement`)))

(event `DamageCoolDown`
  (`KismetSystemLibrary.Delay` 0.2)
  (set `self.CanBeHit?` true))

(event `TakeDamage`
  (params (DamageTaken :type Integer))
  ; Prendre des Dégat
  (if (`self.CanBeHit?`)
    (set `self.CanBeHit?` false)
    (`self.DamageCoolDown`)
    (set `self.Health` (- (`self.Health`) DamageTaken))
    (`KismetSystemLibrary.PrintString` (`KismetTextLibrary.Conv_TextToString` (`|FormatText` "Hit : {Name}" (`self.Name`))))
    (`KismetSystemLibrary.PrintString` (`KismetTextLibrary.Conv_TextToString` (`|FormatText` "Health Left {Health}" (`self.Health`))))))

(fn `UserConstructionScript`
  (set `self.Name` (`.EnemyName_2_7E4648B34DD2A25820EB3B9326B53812` (break `/Game/Blueprints/Enemies/Data/F_EnemyStats` (`/Game/Blueprints/Enemies/Data/PDA_Enemy.EnemyStats` (`self.EnemyStats`))))))