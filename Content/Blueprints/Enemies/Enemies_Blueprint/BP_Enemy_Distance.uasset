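; Ranged enemy, using the Enemy_2 stats entry, that shoots projectiles at the player and backs away when approached.
; Sphere overlap starts the chase behavior tree; straying beyond Range from Anchor switches back to wander.
; Tick sphere traces trigger a montage-and-projectile attack with cooldown, or at closer range a self-repeating AIMoveTo retreat.
; The EnemyFlee tree and FleePLayer toggles are unconnected, so retreat relies on RunAway alone.
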(event `RunAway`
  (bind _returnvalue (`self.K2_GetActorLocation`))
  (`|AIMoveTo` self (`KismetMathLibrary.MakeVector` (.x (+ _returnvalue (* (`KismetMathLibrary.GetForwardVector` (`KismetMathLibrary.FindLookAtRotation` _returnvalue (`self.K2_GetActorLocation` (`self.CharRef`)))) -500.0))) (.y (+ _returnvalue (* (`KismetMathLibrary.GetForwardVector` (`KismetMathLibrary.FindLookAtRotation` _returnvalue (`self.K2_GetActorLocation` (`self.CharRef`)))) -500.0))) (.z _returnvalue)) null
    (:`OnSuccess`
      (`self.RunAway`))))

(event `self.ReceiveTick`
  (params (DeltaSeconds :type "Float (single-precision)"))
  (bind _returnvalue (`self.K2_GetActorLocation`))
  (bind _returnvalue_2 (`self.K2_GetActorLocation`))
  (`parent.ReceiveTick` DeltaSeconds)
  (`|ExecutionSequence`
    (:`then_0`
      (if (not (`self.FleePLayer`))
        ; Ranged Collision
        (bind _outactors (`GameplayStatics.GetAllActorsWithTag` "Enemy"))
        (bind _outhit (`KismetSystemLibrary.SphereTraceSingleForObjects` _returnvalue _returnvalue 600.0 (`|MakeArray` "ObjectTypeQuery3" :!type "EObjectTypeQuery Enum") false _outactors "ForOneFrame" true (struct :`R` 1.0 :`A` 1.0) (struct :`G` 1.0 :`A` 1.0) 0.3))
        (if (== (`.HitActor` (`GameplayStatics.BreakHitResult` _outhit)) (`GameplayStatics.GetPlayerCharacter` 0))
          (`self.RangedAttack`))))
    (:`then_1`
      ; Return to Anchor if out of chase Collision
      (if (`self.IsChasing`)
        (if (> (`KismetMathLibrary.Vector_Distance` (`self.Anchor`) (`self.K2_GetActorLocation`)) (`self.Range`))
          (`self.StopChase`))))
    (:`then_2`
      (bind _outactors_2 (`GameplayStatics.GetAllActorsWithTag` "Enemy"))
      (bind _outhit_2 (`KismetSystemLibrary.SphereTraceSingleForObjects` _returnvalue_2 _returnvalue_2 400.0 (`|MakeArray` "ObjectTypeQuery3" :!type "EObjectTypeQuery Enum") false _outactors_2 "ForOneFrame" true (struct :`R` 1.0 :`A` 1.0) (struct :`G` 1.0 :`A` 1.0) 0.3))
      (if (== (`.HitActor` (`GameplayStatics.BreakHitResult` _outhit_2)) (`GameplayStatics.GetPlayerCharacter` 0))
        (`self.StopChase`)
        (`BlackboardComponent.ClearValue` (`AIBlueprintHelperLibrary.GetBlackboard` (`AIBlueprintHelperLibrary.GetAIController` self)) "TargetActor")
        (`self.RunAway`)))
    (:`then_3`
      (bind _asbp_top_down_character (cast `/Game/Blueprints/Character/BP_TopDownCharacter` (`GameplayStatics.GetPlayerCharacter` 0)))
      (set `self.CharRef` _asbp_top_down_character))))

(event `CoolDown`
  ; Attack CD
  (`KismetSystemLibrary.Delay` 3.0)
  (set `self.CanAttack` true))

(event `RangedAttack`
  (bind _attacking (`self.attacking`))
  ; Ranged Attack
  (if (`self.CanAttack`)
    (set `self.CanAttack` false)
    (`self.CoolDown`)
    (set `CharacterMovementComponent.MaxWalkSpeed` 0.0 (`self.CharacterMovement`))
    (`self.PlayAnimMontage` _attacking)
    (`self.K2_SetActorRotation` (`KismetMathLibrary.FindLookAtRotation` (`self.K2_GetActorLocation`) (`SceneComponent.K2_GetComponentLocation` (`Character.CapsuleComponent` (`GameplayStatics.GetPlayerCharacter` 0)))))
    (`|SpawnActorFromClass` "/Game/Blueprints/Enemies/Enemies_Blueprint/BP_DistanceEnemyProjectile.BP_DistanceEnemyProjectile_C" (`SceneComponent.K2_GetComponentToWorld` (`self.Muzzle`)) "Undefined" "MultiplyWithRoot" null null)
    (`KismetSystemLibrary.Delay` (`AnimSequenceBase.SequenceLength` _attacking))
    (set `CharacterMovementComponent.MaxWalkSpeed` (`self.ChaseSpeed`) (`self.CharacterMovement`))))

(event `StartChase`
  ; Start Chasing Player
  (if (not (`self.IsAttacking`))
    (set `self.IsChasing` true)
    (set `CharacterMovementComponent.MaxWalkSpeed` (`self.ChaseSpeed`) (`self.CharacterMovement`))
    (`AIController.RunBehaviorTree` (`AIBlueprintHelperLibrary.GetAIController` self) "/Game/Blueprints/Enemies/Data/EnemyChase.EnemyChase")
    (`BlackboardComponent.ClearValue` (`AIBlueprintHelperLibrary.GetBlackboard` (`AIBlueprintHelperLibrary.GetAIController` self)) "TargetActor")))

(event `self.Sphere.OnComponentBeginOverlap`
  (params (OverlappedComponent :type "PrimitiveComponent Object Reference") (OtherActor :type "Actor Object Reference") (OtherComp :type "PrimitiveComponent Object Reference") (OtherBodyIndex :type Integer) (bFromSweep :type Boolean) (SweepResult :type "HitResult Structure (by ref)"))
  ; Start Chasing if In sight collision
  (if (== null (`GameplayStatics.GetPlayerCharacter` 0))
    (`self.StartChase`)
    (`BlackboardComponent.SetValueAsObject` (`AIBlueprintHelperLibrary.GetBlackboard` (`AIBlueprintHelperLibrary.GetAIController` self)) "TargetActor" null)))

(event `StopChase`
  ; Stop Chasing Player
  (set `self.IsChasing` false)
  (set `CharacterMovementComponent.MaxWalkSpeed` (`self.WalkSpeed`) (`self.CharacterMovement`))
  (`AIController.RunBehaviorTree` (`AIBlueprintHelperLibrary.GetAIController` self) "/Game/Blueprints/Enemies/Data/EnemyWander.EnemyWander"))

(fn `UserConstructionScript`
  (set `self.EnemyStats` "/Game/Blueprints/Enemies/Data/Enemy_2.Enemy_2")
  (`parent.UserConstructionScript`))