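; Melee enemy that wanders, chases the player on entering its sight sphere, and attacks up close.
; Switches between EnemyChase and EnemyWander behavior trees and speeds, giving up chase beyond Range from its Anchor.
; Tick runs a sphere trace that triggers a montage attack, halting movement while it plays, and destroys the actor at zero Health.
; Construction assigns the Enemy_1 stats; CanAttack is cleared on attack and not reset here.
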(event `StartChase`
  ; Commencer Chase player
  (if (not (`self.IsAttacking`))
    (set `self.IsChasing` true)
    (set `CharacterMovementComponent.MaxWalkSpeed` (`self.ChaseSpeed`) (`self.CharacterMovement`))
    (`AIController.RunBehaviorTree` (`AIBlueprintHelperLibrary.GetAIController` self) "/Game/Blueprints/Enemies/Data/EnemyChase.EnemyChase")
    (`BlackboardComponent.ClearValue` (`AIBlueprintHelperLibrary.GetBlackboard` (`AIBlueprintHelperLibrary.GetAIController` self)) "TargetActor")))

(event `self.Sphere.OnComponentBeginOverlap`
  (params (OverlappedComponent :type "PrimitiveComponent Object Reference") (OtherActor :type "Actor Object Reference") (OtherComp :type "PrimitiveComponent Object Reference") (OtherBodyIndex :type Integer) (bFromSweep :type Boolean) (SweepResult :type "HitResult Structure (by ref)"))
  ; Sight Range
  (if (== OtherActor (`GameplayStatics.GetPlayerCharacter` 0))
    (`self.StartChase`)
    (`BlackboardComponent.SetValueAsObject` (`AIBlueprintHelperLibrary.GetBlackboard` (`AIBlueprintHelperLibrary.GetAIController` self)) "TargetActor" OtherActor)))

(event `StopChase`
  ; Arreter chase player
  (set `self.IsChasing` false)
  (set `CharacterMovementComponent.MaxWalkSpeed` (`self.WalkSpeed`) (`self.CharacterMovement`))
  (`AIController.RunBehaviorTree` (`AIBlueprintHelperLibrary.GetAIController` self) "/Game/Blueprints/Enemies/Data/EnemyWander.EnemyWander"))

(event `self.AttackCollision.OnComponentBeginOverlap`
  (params (OverlappedComponent :type "PrimitiveComponent Object Reference") (OtherActor :type "Actor Object Reference") (OtherComp :type "PrimitiveComponent Object Reference") (OtherBodyIndex :type Integer) (bFromSweep :type Boolean) (SweepResult :type "HitResult Structure (by ref)"))
  ; Attack Collision
  (if (== OtherActor (`GameplayStatics.GetPlayerCharacter` 0))
    (set `self.IsAttacking` true)))

(event `self.ReceiveTick`
  (params (DeltaSeconds :type "Float (single-precision)"))
  ; Detection si le joueur est en distance d'attaque
  (`parent.ReceiveTick` DeltaSeconds)
  (`|ExecutionSequence`
    (:`then_0`
      (bind _outactors (`GameplayStatics.GetAllActorsWithTag` "Enemy"))
      (bind _outhit (`KismetSystemLibrary.SphereTraceSingleForObjects` (`SceneComponent.K2_GetComponentLocation` (`self.Begin`)) (`SceneComponent.K2_GetComponentLocation` (`self.End`)) 80.0 (`|MakeArray` "ObjectTypeQuery3" :!type "EObjectTypeQuery Enum") false _outactors "None" true (struct :`R` 1.0 :`A` 1.0) (struct :`G` 1.0 :`A` 1.0) 0.3))
      (if (== (`.HitActor` (`GameplayStatics.BreakHitResult` _outhit)) (`GameplayStatics.GetPlayerCharacter` 0))
        (`self.BeginAttack`)))
    (:`then_1`
      (if (`self.IsChasing`)
        (if (> (`KismetMathLibrary.Vector_Distance` (`self.Anchor`) (`self.K2_GetActorLocation`)) (`self.Range`))
          (`self.StopChase`))))
    (:`then_2`
      (if (<= (`self.Health`) 0)
        (`self.K2_DestroyActor`)))))

(event `self.AttackCollision.OnComponentEndOverlap`
  (params (OverlappedComponent :type "PrimitiveComponent Object Reference") (OtherActor :type "Actor Object Reference") (OtherComp :type "PrimitiveComponent Object Reference") (OtherBodyIndex :type Integer))
  ; Attack Collision
  (if (== OtherActor (`GameplayStatics.GetPlayerCharacter` 0))
    (set `self.IsAttacking` false)))

(event `BeginAttack`
  ; Jouer l'anim + collision d'attaque
  (if (`self.CanAttack`)
    (set `self.CanAttack` false)
    (set `CharacterMovementComponent.MaxWalkSpeed` 0.0 (`self.CharacterMovement`))
    (bind _returnvalue (`self.PlayAnimMontage` (`self.attacking`)))
    (`KismetSystemLibrary.Delay` _returnvalue)
    (set `CharacterMovementComponent.MaxWalkSpeed` (`self.ChaseSpeed`) (`self.CharacterMovement`))))

(fn `UserConstructionScript`
  (set `self.EnemyStats` "/Game/Blueprints/Enemies/Data/Enemy_1.Enemy_1")
  (`parent.UserConstructionScript`))