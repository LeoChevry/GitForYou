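; Base enemy character that chases the player, takes damage and drops items on death.
; Construction loads stats from EnemyStats and sizes the detection sphere to Range.
; Sphere overlap starts chase, setting speed and blackboard target; Tick stops it beyond Range, though both states run EnemyChase.
; TakeDamage flashes the material but has an unreset DoOnce; zero health triggers random drops, then destruction.
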(event `self.ReceiveBeginPlay`
  (set `self.BaseMaterials` (`PrimitiveComponent.GetMaterial` (`self.Mesh`) 0)))

(event `self.Sphere.OnComponentBeginOverlap`
  (params (OverlappedComponent :type "PrimitiveComponent Object Reference") (OtherActor :type "Actor Object Reference") (OtherComp :type "PrimitiveComponent Object Reference") (OtherBodyIndex :type Integer) (bFromSweep :type Boolean) (SweepResult :type "HitResult Structure (by ref)"))
  (if (== OtherActor (`GameplayStatics.GetPlayerCharacter` 0))
    (`self.StartChase`)
    (`BlackboardComponent.SetValueAsObject` (`AIBlueprintHelperLibrary.GetBlackboard` (`AIBlueprintHelperLibrary.GetAIController` self)) "TargetActor" OtherActor)))

(event `self.ReceiveTick`
  (params (DeltaSeconds :type "Float (single-precision)"))
  (`|ExecutionSequence`
    (:`then_0`
      (if (`self.IsChasing`)
        (if (> (`KismetMathLibrary.Vector_Distance` (`self.K2_GetActorLocation`) (`self.K2_GetActorLocation` (`GameplayStatics.GetPlayerCharacter` 0))) (`self.Range`))
          (`self.StopChase`))))
    (:`then_1`
      (if (<= (`self.Health`) 0)
        (`|ExecutionSequence`
          (:`then_0`
            (`self.DropItem`))
          (:`then_1`
            (`KismetSystemLibrary.Delay` 0.1)
            (`self.K2_DestroyActor`)))))))

(event `StartChase`
  (set `self.IsChasing` true)
  (set `CharacterMovementComponent.MaxWalkSpeed` 500.0 (`self.CharacterMovement`))
  (`AIController.RunBehaviorTree` (`AIBlueprintHelperLibrary.GetAIController` self) "/Game/Blueprints/Enemies/Data/EnemyChase.EnemyChase"))

(event `StopChase`
  (set `self.IsChasing` false)
  (set `CharacterMovementComponent.MaxWalkSpeed` 300.0 (`self.CharacterMovement`))
  (`AIController.RunBehaviorTree` (`AIBlueprintHelperLibrary.GetAIController` self) "/Game/Blueprints/Enemies/Data/EnemyChase.EnemyChase"))

(event `TakeDamage`
  (params (Damage :type Integer))
  (bind _mesh (`self.Mesh`))
  (`/Engine/EditorBlueprintResources/StandardMacros.DoOnce` false
    (:`Completed`
      (set `self.Health` (- (`self.Health`) Damage))
      (`PrimitiveComponent.SetMaterial` _mesh 0 "/Engine/MapTemplates/Materials/BasicAsset03.BasicAsset03")
      (`KismetSystemLibrary.Delay` 0.3)
      (`PrimitiveComponent.SetMaterial` _mesh 0 (`self.BaseMaterials`)))))

(event `DropItem`
  (`/Engine/EditorBlueprintResources/StandardMacros.DoOnce` false
    (:`Completed`
      (for _index (range (+ (`KismetMathLibrary.RandomIntegerInRange` (`self.MinDrop`) (`self.MaxDrop`)) 1))
        (`|SpawnActorFromClass` "/Game/Blueprints/Enemies/BP_TEMP_Drop.BP_TEMP_Drop_C" (`KismetMathLibrary.MakeTransform` (`self.K2_GetActorLocation`)) "Undefined" "MultiplyWithRoot" null false null))
      (`KismetSystemLibrary.PrintString` (`KismetStringLibrary.Conv_IntToString` _index)))))

(fn `UserConstructionScript`
  (bind (_enemyname _enemymesh _enemyhealth _enemyspeed _enemydef _enemydamage _enemyatkspeed _enemycollisionsize _mindrop _maxdrop) (break `/Game/Blueprints/Enemies/Data/F_EnemyStats` (`/Game/Blueprints/Enemies/Data/PDA_Enemy.EnemyStats` (`self.EnemyStats`))))
  (set `self.Name` _enemyname)
  (set `self.Health` _enemyhealth)
  (`CapsuleComponent.SetCapsuleSize` (`self.CapsuleComponent`) 34.0 96.0 true)
  (set `self.MinDrop` _mindrop)
  (set `self.MaxDrop` _maxdrop)
  (`SphereComponent.SetSphereRadius` (`self.Sphere`) (`self.Range`) true))