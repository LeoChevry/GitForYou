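; Test enemy actor, configured from EnemyStats data, that takes damage and drops items on death.
; The construction script copies name, mesh, health, collision box size and drop range from those stats.
; TakeDamage lowers Health, and Tick polls for zero to trigger DropItem and a briefly delayed destroy.
; DropItem uses DoOnce to spawn BP_TEMP_Drop actors in a zero-to-random inclusive loop at the enemy's location.
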(event `self.ReceiveTick`
  (params (DeltaSeconds :type "Float (single-precision)"))
  ; Mort
  (if (<= (`self.Health`) 0)
    (`|ExecutionSequence`
      (:`then_0`
        (`self.DropItem`))
      (:`then_1`
        (`KismetSystemLibrary.Delay` 0.1)
        (`self.K2_DestroyActor`)))))

(event `DropItem`
  ; Drop des Items un nombre X de fois
  (`/Engine/EditorBlueprintResources/StandardMacros.DoOnce` false
    (:`Completed`
      (for _index (range (+ (`KismetMathLibrary.RandomIntegerInRange` (`self.Min Drop`) (`self.Max Drop`)) 1))
        (`|SpawnActorFromClass` "/Game/Blueprints/Enemies/BP_TEMP_Drop.BP_TEMP_Drop_C" (`KismetMathLibrary.MakeTransform` (`self.K2_GetActorLocation`)) "Undefined" "MultiplyWithRoot" null null))
      (`KismetSystemLibrary.PrintString` (`KismetStringLibrary.Conv_IntToString` _index)))))

(event `self.ReceiveBeginPlay`)

(event `TakeDamage`
  (params (Damage :type Integer))
  ; Prendre des Dégats
  (set `self.Health` (- (`self.Health`) Damage)))

(fn `UserConstructionScript`
  (bind (_enemyname _enemymesh _enemyhealth _enemyspeed _enemydef _enemydamage _enemyatkspeed _enemycollisionsize _mindrop _maxdrop) (break `/Game/Blueprints/Enemies/Data/F_EnemyStats` (`/Game/Blueprints/Enemies/Data/PDA_Enemy.EnemyStats` (`self.EnemyStats`))))
  (set `self.Name` _enemyname)
  (`StaticMeshComponent.SetStaticMesh` (`self.StaticMesh`) _enemymesh)
  (set `self.Health` _enemyhealth)
  (`BoxComponent.SetBoxExtent` (`self.Collision`) _enemycollisionsize true)
  (set `self.Min Drop` _mindrop)
  (set `self.Max Drop` _maxdrop))