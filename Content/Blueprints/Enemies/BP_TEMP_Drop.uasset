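; BP_TEMP_Drop is an item drop pickup that pops out with a random physics impulse on spawn, unless flagged as dropped.
; Overlapping AttractRange moves it toward the top-down character, except during the cooldown after being dropped.
; GrabCollision overlap passes the character to ItemDataComponent.InteractWith, then destroys the actor, regardless of cooldown.
; LookAt builds a pickup prompt from the item's data table name.
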(event `DropCoolDown`
  ; Cooldown quand L'item a été drop
  (`KismetSystemLibrary.Delay` 6.0)
  (set `self.HasBeenDropped?` false))

(event `self.ReceiveBeginPlay`
  (bind _returnvalue (`KismetMathLibrary.RandomFloatInRange` 0.0 1.0))
  ; Rebond lors de l'instanciate de l'Item
  (if (`self.HasBeenDropped?`)
    (`self.DropCoolDown`)
    (else
      (`PrimitiveComponent.AddImpulse` (`self.StaticMesh`) (* (`KismetMathLibrary.MakeVector` 0.0 _returnvalue _returnvalue) 500.0) "None" false))))

(event `self.AttractRange.OnComponentBeginOverlap`
  (params (OverlappedComponent :type "PrimitiveComponent Object Reference") (OtherActor :type "Actor Object Reference") (OtherComp :type "PrimitiveComponent Object Reference") (OtherBodyIndex :type Integer) (bFromSweep :type Boolean) (SweepResult :type "HitResult Structure (by ref)"))
  ; Range du pickup
  (bind _asbp_top_down_character (cast `/Game/Blueprints/Character/BP_TopDownCharacter` OtherActor))
  (if (not (`self.HasBeenDropped?`))
    (`KismetSystemLibrary.MoveComponentTo` (`self.DefaultSceneRoot`) (`self.K2_GetActorLocation` _asbp_top_down_character) (struct) false true)))

(event `self.GrabCollision.OnComponentBeginOverlap`
  (params (OverlappedComponent :type "PrimitiveComponent Object Reference") (OtherActor :type "Actor Object Reference") (OtherComp :type "PrimitiveComponent Object Reference") (OtherBodyIndex :type Integer) (bFromSweep :type Boolean) (SweepResult :type "HitResult Structure (by ref)"))
  ; Range du pickup
  ;; Ajouter à l'inventaire
  (bind _asbp_top_down_character (cast `/Game/Blueprints/Character/BP_TopDownCharacter` OtherActor))
  (`/Engine/EditorBlueprintResources/StandardMacros.IsValid` _asbp_top_down_character
    (:`Is Valid`
      (`/Game/Blueprints/Character/Inventory/I_InteractInterface.InteractWith` (`self.ItemDataComponent`) _asbp_top_down_character)
      (`self.K2_DestroyActor`))))

(fn `LookAt`
  (returns (Message :type Text))
  (bind (_itemid_datatable _itemid_rowname) (break `DataTableRowHandle` (`/Game/Blueprints/Character/Inventory/ItemDataComponent.ItemID` (`self.ItemDataComponent`))))
  (bind _returnvalue (`|GetDataTableRow` _itemid_datatable _itemid_rowname)
    (:`then`
      (return (`|FormatText` "Pick up {item}" (`.Name_5_A0DB97A94185298E31060AB52ABC7589` (break `/Game/Blueprints/Character/Inventory/F_ItemStruct` _returnvalue)))))))

(fn `UserConstructionScript`)