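; BP_TestEnemy is a data-driven test enemy with health, a static mesh and box collision.
; Its construction script copies name, mesh, health and collision size from EnemyStats.
; TakeDamage subtracts health and prints name and remaining health.
; Tick polls for zero health, calling DropItem (an empty stub, like SetupEnemy) each frame until a short delay ends in DestroyActor.
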(event `self.ReceiveTick`
  (params (DeltaSeconds :type "Float (single-precision)"))
  (if (<= (`self.Health`) 0)
    (`self.DropItem`)
    (`KismetSystemLibrary.Delay` 0.1)
    (`self.K2_DestroyActor`)))

(event `DropItem`)

(event `self.ReceiveBeginPlay`)

(event `TakeDamage`
  (params (Damage :type Integer))
  (bind _output_get (set `self.Health` (- (`self.Health`) Damage)))
  (`KismetSystemLibrary.PrintString` (`KismetStringLibrary.Conv_NameToString` (`self.Name`)))
  (`KismetSystemLibrary.PrintString` (`KismetStringLibrary.Conv_IntToString` _output_get)))

(event `SetupEnemy`)

(fn `UserConstructionScript`
  (bind (_enemyname _enemymesh _enemyhealth _enemyspeed _enemydef _enemydamage _enemyatkspeed _enemycollisionsize) (break `/Game/Blueprints/Enemies/F_EnemyStats` (`/Game/Blueprints/Enemies/PDA_Enemy.EnemyStats` (`self.EnemyStats`))))
  (set `self.Name` _enemyname)
  (`StaticMeshComponent.SetStaticMesh` (`self.StaticMesh`) _enemymesh)
  (set `self.Health` _enemyhealth)
  (`BoxComponent.SetBoxExtent` (`self.Collision`) _enemycollisionsize true))