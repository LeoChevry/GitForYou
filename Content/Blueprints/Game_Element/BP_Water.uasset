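; Water volume actor that slows the top-down character and puts out any fire it carries.
; Overlapping the water mesh lowers walk speed and clears the character's fire state, and leaving restores a fixed walk speed.
; DryWater and UndryWater events slide the mesh over one second to the DryPosition component's transform or back to zero relative location and rotation.
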(event `self.WaterMesh.OnComponentBeginOverlap`
  (params (OverlappedComponent :type "PrimitiveComponent Object Reference") (OtherActor :type "Actor Object Reference") (OtherComp :type "PrimitiveComponent Object Reference") (OtherBodyIndex :type Integer) (bFromSweep :type Boolean) (SweepResult :type "HitResult Structure (by ref)"))
  (bind _asbp_top_down_character (cast `/Game/Blueprints/Character/BP_TopDownCharacter` OtherActor))
  (set `CharacterMovementComponent.MaxWalkSpeed` 300.0 (`Character.CharacterMovement` _asbp_top_down_character))
  (if (`/Game/Blueprints/Character/BP_TopDownCharacter.HasFire` _asbp_top_down_character)
    (`/Game/Blueprints/Character/BP_TopDownCharacter.UpdateFire` _asbp_top_down_character false)
    (`KismetSystemLibrary.PrintString` "Fire extinguished")))

(event `self.WaterMesh.OnComponentEndOverlap`
  (params (OverlappedComponent :type "PrimitiveComponent Object Reference") (OtherActor :type "Actor Object Reference") (OtherComp :type "PrimitiveComponent Object Reference") (OtherBodyIndex :type Integer))
  (bind _asbp_top_down_character (cast `/Game/Blueprints/Character/BP_TopDownCharacter` OtherActor))
  (set `CharacterMovementComponent.MaxWalkSpeed` 600.0 (`Character.CharacterMovement` _asbp_top_down_character)))

(event `DryWater`
  (bind _dryposition (`self.DryPosition`))
  (`KismetSystemLibrary.MoveComponentTo` (`self.WaterMesh`) (`SceneComponent.RelativeLocation` _dryposition) (`SceneComponent.RelativeRotation` _dryposition) false false 1.0)
  (`KismetSystemLibrary.PrintString` "Hello"))

(event `UndryWater`
  (`KismetSystemLibrary.MoveComponentTo` (`self.WaterMesh`) (0.0 0.0 0.0) (struct) false false 1.0))

(fn `UserConstructionScript`)