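; Fire stele interactable that holds a fire the player can take or return, driving a linked mechanism.
; Interacting moves the fire between stele and player, who carries one at most, and toggles the point light to match.
; The linked mechanism receives Activate(true) when fire is taken and Activate(false) when it is placed or present at BeginPlay.
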(event `self.ReceiveBeginPlay`
  (if (`self.FirePresent`)
    (`LightComponent.SetIntensity` (`self.PointLight`) 5000.0 :!label _label)
    (bind _linkedmechanism (`self.LinkedMechanism`)
      (:`then`
        (`/Game/Blueprints/Game_Element/BP_Mechanism.Activate` _linkedmechanism false))
      (:`else`))))

(event `/Game/Blueprints/Character/Inventory/I_InteractInterface.InteractWith`
  (params (PlayerCharacter :type "/Game/Blueprints/Character/BP_TopDownCharacter Object Reference"))
  (bind _hasfire (`/Game/Blueprints/Character/BP_TopDownCharacter.HasFire` PlayerCharacter))
  (`/Engine/EditorBlueprintResources/StandardMacros.IsValid` PlayerCharacter
    (:`Is Valid`
      (if (`self.FirePresent`)
        (if _hasfire
          (`KismetSystemLibrary.PrintString` "Already have fire")
          (else
            (`KismetSystemLibrary.PrintString` "Fire Taken")
            (`/Game/Blueprints/Character/BP_TopDownCharacter.UpdateFire` PlayerCharacter true)
            (set `self.FirePresent` false)
            (`LightComponent.SetIntensity` (`self.PointLight`) 0.0)
            (bind _linkedmechanism (`self.LinkedMechanism`)
              (:`then`
                (`/Game/Blueprints/Game_Element/BP_Mechanism.Activate` _linkedmechanism true))
              (:`else`))))
        (elif _hasfire
          (`KismetSystemLibrary.PrintString` "Activating")
          (`/Game/Blueprints/Character/BP_TopDownCharacter.UpdateFire` PlayerCharacter false)
          (set `self.FirePresent` true)
          (goto _label)
          (else
            (`KismetSystemLibrary.PrintString` "Can't activate")))))))

(fn `LookAt`
  (returns (Message :type Text))
  (return ""))

(fn `UserConstructionScript`)