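; BP_ItemStack is a world pickup actor that holds items in an InventorySystem component and displays a configurable mesh set at BeginPlay.
; Interactwith uses a FlipFlop to alternately show and remove the inventory as a container on the player controller's HUD.
; When an inventory update leaves the quantity at zero or below, it removes the container and destroys itself.
; LookAt returns a prompt text built from the item's Name.
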(event `self.ReceiveBeginPlay`
  (`StaticMeshComponent.SetStaticMesh` (`self.StaticMesh`) (`self.MeshToSpawn`)))

(event `self.InteractWith`
  (params (PlayerCharacter :type "/Game/Blueprints/Character/BP_TopDownCharacter Object Reference"))
  (`/Engine/EditorBlueprintResources/StandardMacros.FlipFlop`
    (:`A`
      (bind _asbp_third_person_player_controller (cast `/Game/Blueprints/Character/ThirdPerson/Blueprints/BP_ThirdPersonPlayerController` (`GameplayStatics.GetPlayerController` 0)))
      (`/Game/Blueprints/Character/UI/UI_DungeonCrawler.ShowContainer` (`/Game/Blueprints/Character/ThirdPerson/Blueprints/BP_ThirdPersonPlayerController.HUD` _asbp_third_person_player_controller) (`self.InventorySystem`)))
    (:`B`
      (bind _asbp_third_person_player_controller_2 (cast `/Game/Blueprints/Character/ThirdPerson/Blueprints/BP_ThirdPersonPlayerController` (`GameplayStatics.GetPlayerController` 0)))
      (`/Game/Blueprints/Character/UI/UI_DungeonCrawler.RemoveContainer` (`/Game/Blueprints/Character/ThirdPerson/Blueprints/BP_ThirdPersonPlayerController.HUD` _asbp_third_person_player_controller_2)))))

(event `self.InventorySystem.OnInventoryUpdated`
  (if (<= (`/Game/Blueprints/Character/Inventory/InventorySystem.GetQuantity` (`self.InventorySystem`)) 0)
    (bind _asbp_third_person_player_controller (cast `/Game/Blueprints/Character/ThirdPerson/Blueprints/BP_ThirdPersonPlayerController` (`GameplayStatics.GetPlayerController` 0)))
    (`/Game/Blueprints/Character/UI/UI_DungeonCrawler.RemoveContainer` (`/Game/Blueprints/Character/ThirdPerson/Blueprints/BP_ThirdPersonPlayerController.HUD` _asbp_third_person_player_controller))
    (`self.K2_DestroyActor`)))

(fn `LookAt`
  (returns (Message :type Text))
  (return (`|FormatText` "Intégarir : {item}" (`self.Name`))))

(fn `UserConstructionScript`)