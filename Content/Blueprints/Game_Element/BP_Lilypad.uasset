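; BP_Lilypad is a moving platform that rides along splines in a loop at a configurable speed and start time.
; A timeline maps progress to spline distance each update, setting the platform's location and yaw.
; Near designated main-spline points it can stop, or switch once per cycle to a secondary trajectory, restarting the timeline.
; On finishing, it returns to the main trajectory and replays; debug prints report the current trajectory.
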(event `self.ReceiveTick`
  (params (DeltaSeconds :type "Float (single-precision)"))
  (`KismetSystemLibrary.PrintString` (`KismetSystemLibrary.GetDisplayName` (`self.CurrentTrajectory`)) true true (struct :`G` 0.66 :`B` 1.0 :`A` 1.0) 0.0))

(event `self.ReceiveBeginPlay`
  (bind _currenttrajectory (`self.CurrentTrajectory`))
  (set `self.CurrentTrajectory` (`self.MainTrajectory`))
  (`TimelineComponent.SetPlayRate` (`self.T_Moving`) (/ (`self.Speed`) 1.0))
  (bind (_direction _progress) (`Timeline|T_Moving` :`NewTime` (`self.StartTime`) :!via `PlayFromStart`)
    (:`Update`
      (bind _returnvalue (`SplineComponent.GetTransformAtDistanceAlongSpline` _currenttrajectory (`KismetMathLibrary.Lerp` 0.0 (`SplineComponent.GetSplineLength` _currenttrajectory) _progress) "World" false))
      (if (and (== (.location _returnvalue) (`SplineComponent.GetLocationAtSplinePoint` (`self.MainTrajectory`) (`self.StopIndex`) "World") :`ErrorTolerance` 20.0) (`self.ShouldStop`))
        (`TimelineComponent.Stop` (`self.T_Moving`))
        (else
          (if (and (== (`SplineComponent.GetLocationAtSplinePoint` (`self.MainTrajectory`) (`self.BranchingIndex`) "World") (.location _returnvalue) :`ErrorTolerance` 20.0) (`self.ShouldBranch`))
            (`/Engine/EditorBlueprintResources/StandardMacros.DoOnce` false :!label _label
              (:`Completed`
                (set `self.CurrentTrajectory` (`self.SecondaryTrajectory`))
                (`KismetSystemLibrary.PrintString` "branched" true true (struct :`G` 0.66 :`B` 1.0 :`A` 1.0) 1.0)
                (`TimelineComponent.PlayFromStart` (`self.T_Moving`)))))
          (`SceneComponent.K2_SetWorldLocationAndRotation` (`self.Plateform`) (.location _returnvalue) (`KismetMathLibrary.MakeRotator` 0.0 0.0 (.yaw (.rotation _returnvalue))) false false))))
    (:`Finished`
      (set `self.CurrentTrajectory` (`self.MainTrajectory`))
      (`TimelineComponent.PlayFromStart` (`self.T_Moving`))
      (goto _label :!via `Reset`))))

(fn `UserConstructionScript`)