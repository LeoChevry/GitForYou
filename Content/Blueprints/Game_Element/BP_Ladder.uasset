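; BP_Ladder is an interactable ladder that instantly moves the player between its bottom and top positions.
; Overlap of BP_TopDownCharacter with the lower or upper collider sets or clears the Climbing flag.
; Interactwith reads that flag and sets the player's transform to UpPosition when climbing, otherwise DownPosition, with no sweep or climbing animation.
; LookAt returns an empty string.
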(event `/Game/Blueprints/Character/Inventory/I_InteractInterface.InteractWith`
  (params (PlayerCharacter :type "/Game/Blueprints/Character/BP_TopDownCharacter Object Reference"))
  (`self.K2_SetActorTransform` PlayerCharacter (select `bool` (`self.Climbing`) :`false` (`SceneComponent.K2_GetComponentToWorld` (`self.DownPosition`)) :`true` (`SceneComponent.K2_GetComponentToWorld` (`self.UpPosition`))) false false))

(event `self.DownCollider.OnComponentBeginOverlap`
  (params (OverlappedComponent :type "PrimitiveComponent Object Reference") (OtherActor :type "Actor Object Reference") (OtherComp :type "PrimitiveComponent Object Reference") (OtherBodyIndex :type Integer) (bFromSweep :type Boolean) (SweepResult :type "HitResult Structure (by ref)"))
  (cast `/Game/Blueprints/Character/BP_TopDownCharacter` OtherActor)
  (set `self.Climbing` true))

(event `self.UpCollider.OnComponentBeginOverlap`
  (params (OverlappedComponent :type "PrimitiveComponent Object Reference") (OtherActor :type "Actor Object Reference") (OtherComp :type "PrimitiveComponent Object Reference") (OtherBodyIndex :type Integer) (bFromSweep :type Boolean) (SweepResult :type "HitResult Structure (by ref)"))
  (cast `/Game/Blueprints/Character/BP_TopDownCharacter` OtherActor)
  (set `self.Climbing` false))

(fn `LookAt`
  (returns (Message :type Text))
  (return ""))

(fn `UserConstructionScript`)