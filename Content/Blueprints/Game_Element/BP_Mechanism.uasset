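; Interactable mechanism that moves its mesh to an end position and changes lily pad and water states, triggered manually or through Activate.
; A timeline scaled by Speed lerps the mesh from its start transform to the hidden EndDestination marker.
; On finish, it sets branch or stop flags on the linked lily pad and dries or blocks linked water.
; Deactivation reverses the timeline and reverts those effects.
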(event `self.ReceiveBeginPlay`
  (`SceneComponent.SetVisibility` (`self.EndDestination`) false false)
  (set `self.StartTransform` (`SceneComponent.GetRelativeTransform` (`self.Mesh`))))

(event `/Game/Blueprints/Character/Inventory/I_InteractInterface.InteractWith`
  (params (PlayerCharacter :type "/Game/Blueprints/Character/BP_TopDownCharacter Object Reference"))
  (if (`self.Manual`)
    (`TimelineComponent.SetPlayRate` (`self.T_Moving`) (/ (`self.Speed`) 1.0) :!label _label)
    (bind (_direction _progress) (`Timeline|T_Moving` :!label _label_2)
      (:`Update`
        (`SceneComponent.K2_SetRelativeTransform` (`self.Mesh`) (`KismetMathLibrary.TLerp` (`self.StartTransform`) (`SceneComponent.GetRelativeTransform` (`self.EndDestination`)) _progress) false false))
      (:`Finished`
        (`|ExecutionSequence`
          (:`then_0`
            ; Branch/block lilypad
            (bind _lilypadref (`self.LilyPadRef`)
              (:`then`
                (`|ExecutionSequence`
                  (:`then_0`
                    (if (`self.AffectBranch`)
                      (bind _returnvalue (not (stale `Activate` Desactiavte)))
                      (set `/Game/Blueprints/Game_Element/BP_Lilypad.ShouldBranch` _returnvalue _lilypadref)))
                  (:`then_1`
                    (if (`self.AffectStop`)
                      (set `/Game/Blueprints/Game_Element/BP_Lilypad.ShouldStop` _returnvalue _lilypadref)
                      (set `/Game/Blueprints/Game_Element/BP_Lilypad.StopIndex` (`self.Stop Index`) _lilypadref)))))
              (:`else`)))
          (:`then_1`
            (for _array_element (`self.WaterToDry`)
              (if (stale `Activate` Desactiavte)
                (if (`/Game/Blueprints/Game_Element/BP_Water.Is block` _array_element)
                  (set `/Game/Blueprints/Game_Element/BP_Water.Is block` false _array_element)
                  (else
                    (`/Game/Blueprints/Game_Element/BP_Water.UndryWater` _array_element)))
                (else
                  (if (`self.Block Water`)
                    (set `/Game/Blueprints/Game_Element/BP_Water.Is block` true _array_element))
                  (`/Game/Blueprints/Game_Element/BP_Water.DryWater` _array_element))))))))))

(event `Activate`
  (params (Desactiavte :type Boolean))
  (if Desactiavte
    (goto _label_2 :!via `Reverse`)
    (else
      (goto _label))))

(fn `LookAt`
  (returns (Message :type Text))
  (return ""))

(fn `UserConstructionScript`)