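; Player pawn for the cookery gameplay, which creates the HUD, handles station changes and lets the player interact with meals and clients.
; Grab traces toward the cursor to pick up a meal or talk to a client; pressing again drops the held meal.
; Tick keeps held meals at the cursor hit, pulled toward the camera and yawed relative to the pawn, with physics off until dropped.
; Events swap station messages and update the HUD's gold display.
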(event `self.ReceiveBeginPlay`
  (bind _returnvalue (`|CreateWidget` "/Game/Blueprints/UI/WBP_CookeryHUD.WBP_CookeryHUD_C"))
  (bind _output_get (set `self.CookeryHUD Ref` _returnvalue))
  (`UserWidget.AddToViewport` _output_get 0))

(event `ChangeStation`
  (params (CurrentStation :type Integer))
  (bind _currentstationwidget (`self.CurrentStationWidget`))
  ; Station Swapper
  (`/Engine/EditorBlueprintResources/StandardMacros.IsValid` _currentstationwidget
    (:`Is Valid`
      (`Widget.RemoveFromParent` _currentstationwidget)
      (set `self.CurrentStationWidget` null))
    (:`Is Not Valid`
      _))
  (switch `int` CurrentStation
    (:`0`
      (set `self.CurrentStation` "/Game/Blueprints/Cooking/BP_Stations.BP_Stations_C"))
    (:`1`
      (set `self.CurrentStation` "/Game/Blueprints/Cooking/BP_CookingStation.BP_CookingStation_C"))
    (:`2`
      (set `self.CurrentStation` "/Game/Blueprints/Cooking/BP_ServiceStation.BP_ServiceStation_C"))
    (:`3`
      (set `self.CurrentStation` null)))
  (bind _returnvalue (`GameplayStatics.GetActorOfClass` (`self.CurrentStation`)))
  (message `/Game/Blueprints/System/BPI_Stations.SetStation` _returnvalue))

(event `self.ReceiveTick`
  (params (DeltaSeconds :type "Float (single-precision)"))
  (bind _objecttomove (`self.ObjectToMove`))
  (bind (_returnvalue_roll _returnvalue_pitch _returnvalue_yaw) (`KismetMathLibrary.BreakRotator` (`KismetMathLibrary.FindLookAtRotation` (`self.K2_GetActorLocation` _objecttomove) (`self.K2_GetActorLocation`))))
  ; Move/rotate Object
  (if (!= (`self.ObjectToMove`) null)
    (`/Engine/EditorBlueprintResources/StandardMacros.IsValid` _objecttomove
      (:`Is Valid`
        (`self.K2_SetActorLocationAndRotation` _objecttomove (+ (`.Location` (`GameplayStatics.BreakHitResult` (`PlayerController.GetHitResultUnderCursorByChannel` (`GameplayStatics.GetPlayerController` 0) "TraceTypeQuery1" true))) (* (`KismetMathLibrary.GetForwardVector` (`PlayerCameraManager.GetCameraRotation` (`GameplayStatics.GetPlayerCameraManager` 0))) -30.0)) (`KismetMathLibrary.MakeRotator` 0.0 0.0 (+ _returnvalue_yaw 90.0)) false false)))))

(event `EnhancedInput|/Game/Input/Actions/IA_Grab`
  (params (ActionValue :type Boolean) (ElapsedSeconds :type "Float (double-precision)") (TriggeredSeconds :type "Float (double-precision)") (InputAction :type "InputAction Object Reference" :default "/Game/Input/Actions/IA_Grab.IA_Grab"))
  (bind _objecttomove (`self.ObjectToMove`))
  (:`Started`
    (`/Engine/EditorBlueprintResources/StandardMacros.IsValid` _objecttomove ; Holding something ?
      (:`Is Valid`
        ; Drop
        (`PrimitiveComponent.SetSimulatePhysics` (`self.GetComponentByClass` _objecttomove "/Script/Engine.SphereComponent") true)
        (set `self.ObjectToMove` null)
        (set `self.SelectedMeal` null))
      (:`Is Not Valid`
        ; Grab
        (bind _outhit (`KismetSystemLibrary.LineTraceSingle` :`Start` (`self.K2_GetActorLocation`) :`End` (`.Location` (`GameplayStatics.BreakHitResult` (`PlayerController.GetHitResultUnderCursorByChannel` (`GameplayStatics.GetPlayerController` 0) "TraceTypeQuery1" true))) :`TraceChannel` "TraceTypeQuery2" :`DrawDebugType` "ForOneFrame"))
        (bind (_bblockinghit _binitialoverlap _time _distance _location _impactpoint _normal _impactnormal _physmat _hitactor) (`GameplayStatics.BreakHitResult` _outhit))
        (bind _asbp_meal (cast `/Game/Blueprints/Cooking/Meal/BP_meal` _hitactor)
          (:`then`
            (bind _output_get (set `self.SelectedMeal` _asbp_meal))
            (set `self.ObjectToMove` _output_get)
            (`PrimitiveComponent.SetSimulatePhysics` (`self.GetComponentByClass` (`self.ObjectToMove`) "/Script/Engine.SphereComponent") false))
          (:`CastFailed`
            (bind _asbp_client (cast `/Game/Blueprints/Cooking/BP_client` _hitactor))
            (if (`/Game/Blueprints/Cooking/BP_client.CanTalk` _asbp_client)
              (`/Game/Blueprints/Cooking/BP_client.Talk` _asbp_client))))))))

(event `UpdateGold`
  (params (GoldToAdd :type Integer))
  (`/Game/Blueprints/UI/WBP_CookeryHUD.UpdateGoldUI` (`self.CookeryHUD Ref`) (+ GoldToAdd (`self.CurrentGold`))))

(fn `UserConstructionScript`)