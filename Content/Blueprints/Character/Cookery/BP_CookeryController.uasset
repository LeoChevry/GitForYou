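; BP_CookeryController is the controller for the cookery gameplay, switching the player's view between four station cameras.
; On BeginPlay it adds the IMC_Cookery input mapping context and views the first camera.
; IA_Rotate steps the camera index forward or back by input sign, wrapping at both ends.
; ChangeCamera then blends to the selected camera and passes the index to BP_CookeryPawn's ChangeStation.
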(event `self.ReceiveBeginPlay`
  (`EnhancedInputSubsystemInterface.AddMappingContext` (subsystem `EnhancedInputLocalPlayerSubsystem`) "/Game/Input/IMC_Cookery.IMC_Cookery" 0 (struct))
  (`self.SetViewTargetWithBlend` (`|ConvertAsset` (`|GetArrayItem` (`self.Cameras`)))))

(event `EnhancedInput|/Game/Input/Actions/IA_Rotate`
  (params (ActionValue :type "Float (double-precision)") (ElapsedSeconds :type "Float (double-precision)") (TriggeredSeconds :type "Float (double-precision)") (InputAction :type "InputAction Object Reference" :default "/Game/Input/Actions/IA_Rotate.IA_Rotate"))
  (bind _returnvalue (+ (`self.CameraIndex`) -1))
  (bind _returnvalue_2 (+ (`self.CameraIndex`) 1))
  (:`Started`
    (`/Engine/EditorBlueprintResources/StandardMacros.CompareFloat` ActionValue
      (:`>`
        (if (> _returnvalue_2 3)
          (set `self.CameraIndex` 0)
          (else
            (set `self.CameraIndex` _returnvalue_2))))
      (:`<`
        (if (< _returnvalue 0)
          (set `self.CameraIndex` 3)
          (else
            (set `self.CameraIndex` _returnvalue)))))
    (`self.Change Camera`)))

(event `Change Camera`
  (`self.SetViewTargetWithBlend` (`|ConvertAsset` (`|GetArrayItem` (`self.Cameras`) (`self.CameraIndex`))) 1.0)
  (bind _asbp_cookery_pawn (cast `/Game/Blueprints/Character/Cookery/BP_CookeryPawn` (`GameplayStatics.GetPlayerPawn` 0)))
  (`/Game/Blueprints/Character/Cookery/BP_CookeryPawn.ChangeStation` _asbp_cookery_pawn (`self.CameraIndex`)))

(fn `UserConstructionScript`)