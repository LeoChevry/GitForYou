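; Player pawn for the cookery, handling station UI and cursor-driven handling of ingredients and meals.
; Changing station clears the current widget and, for station 1, opens the cook inventory, while a spawn event creates the chosen ingredient under the cursor, already held.
; Grab toggles between line-trace pickup and physics drop, with Tick moving held objects to the cursor hit point plus an offset.
; Retrieve returns a held ingredient's data to the inventory and destroys its actor.
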(event `ChangeStation`
  (params (CurrentStation :type Integer))
  (bind _currentwidget (`self.CurrentWidget`))
  ; Station Swapper
  (`/Engine/EditorBlueprintResources/StandardMacros.IsValid` _currentwidget
    (:`Is Valid`
      (`Widget.RemoveFromParent` _currentwidget)
      (set `self.CurrentWidget` null))
    (:`Is Not Valid`
      _))
  (switch `int` CurrentStation
    (:`1`
      (bind _returnvalue (`|CreateWidget` "/Game/Blueprints/UI/WBP_CookInventory.WBP_CookInventory_C"))
      (bind _output_get (set `self.CurrentWidget` _returnvalue))
      (`UserWidget.AddToViewport` _output_get 0)
      (`/Game/Blueprints/UI/WBP_CookInventory.UpdateInventory` _returnvalue (`/Game/Blueprints/UI/WBP_CookInventory.Cookery Inventory` _returnvalue)))))

(event `SpawnSelectedIngredient`
  (params (IngredientStat :type "/Game/Blueprints/System/PDA_Ingredient Object Reference"))
  ; Spawn Ingreddient
  (bind _returnvalue (`|SpawnActorFromClass` "/Game/Blueprints/Cooking/Ingredients/BP_Ingredient.BP_Ingredient_C" (`KismetMathLibrary.Conv_VectorToTransform` (`.Location` (`GameplayStatics.BreakHitResult` (`PlayerController.GetHitResultUnderCursorByChannel` (`GameplayStatics.GetPlayerController` 0) "TraceTypeQuery1" true)))) "Undefined" "MultiplyWithRoot" null IngredientStat null))
  (bind _output_get (set `self.SelectedIngredient` _returnvalue))
  (set `self.ObjectToMove` _output_get))

(event `self.ReceiveTick`
  (params (DeltaSeconds :type "Float (single-precision)"))
  (bind _objecttomove (`self.ObjectToMove`))
  (bind _selectedmeal (`self.SelectedMeal`))
  (bind _returnvalue (+ (`.Location` (`GameplayStatics.BreakHitResult` (`PlayerController.GetHitResultUnderCursorByChannel` (`GameplayStatics.GetPlayerController` 0) "TraceTypeQuery1" true))) (0.0 -30.0 0.0)))
  ; Move Object
  (if (!= (`self.SelectedIngredient`) null)
    (`/Engine/EditorBlueprintResources/StandardMacros.IsValid` _objecttomove
      (:`Is Valid`
        (`self.K2_SetActorLocation` _objecttomove _returnvalue false false)
        (`/Engine/EditorBlueprintResources/StandardMacros.IsValid` _selectedmeal
          (:`Is Valid`
            (`self.K2_SetActorLocation` _selectedmeal _returnvalue false false)))))))

(event `EnhancedInput|/Game/Input/Actions/IA_Grab`
  (params (ActionValue :type Boolean) (ElapsedSeconds :type "Float (double-precision)") (TriggeredSeconds :type "Float (double-precision)") (InputAction :type "InputAction Object Reference" :default "/Game/Input/Actions/IA_Grab.IA_Grab"))
  (bind _objecttomove (`self.ObjectToMove`))
  (:`Started`
    (`/Engine/EditorBlueprintResources/StandardMacros.IsValid` _objecttomove ; Holding something ?
      (:`Is Valid`
        ; Drop
        (`PrimitiveComponent.SetSimulatePhysics` (`self.GetComponentByClass` _objecttomove "/Script/Engine.SphereComponent") true)
        (set `self.ObjectToMove` null)
        (set `self.SelectedIngredient` null)
        (set `self.SelectedMeal` null))
      (:`Is Not Valid`
        ; Grab
        (bind _outhit (`KismetSystemLibrary.LineTraceSingle` :`Start` (`self.K2_GetActorLocation`) :`End` (`.Location` (`GameplayStatics.BreakHitResult` (`PlayerController.GetHitResultUnderCursorByChannel` (`GameplayStatics.GetPlayerController` 0) "TraceTypeQuery1" true))) :`TraceChannel` "TraceTypeQuery2" :`DrawDebugType` "ForOneFrame"))
        (bind (_bblockinghit _binitialoverlap _time _distance _location _impactpoint _normal _impactnormal _physmat _hitactor) (`GameplayStatics.BreakHitResult` _outhit))
        (bind _asbp_ingredient (cast `/Game/Blueprints/Cooking/Ingredients/BP_Ingredient` _hitactor)
          (:`then`
            (bind _output_get (set `self.SelectedIngredient` _asbp_ingredient))
            (set `self.ObjectToMove` _output_get))
          (:`CastFailed`
            (bind _asbp_meal (cast `/Game/Blueprints/Cooking/Meal/BP_meal` _hitactor))
            (bind _output_get_2 (set `self.SelectedMeal` _asbp_meal))
            (set `self.ObjectToMove` _output_get_2)))
        (`PrimitiveComponent.SetSimulatePhysics` (`self.GetComponentByClass` (`self.ObjectToMove`) "/Script/Engine.SphereComponent") false)))))

(event `EnhancedInput|/Game/Input/Actions/IA_Retrieve`
  (params (ActionValue :type Boolean) (ElapsedSeconds :type "Float (double-precision)") (TriggeredSeconds :type "Float (double-precision)") (InputAction :type "InputAction Object Reference" :default "/Game/Input/Actions/IA_Retrieve.IA_Retrieve"))
  (bind _selectedingredient (`self.SelectedIngredient`))
  ; Retrieve holded ingredient in inventory
  (:`Started`
    (`/Engine/EditorBlueprintResources/StandardMacros.IsValid` _selectedingredient
      (:`Is Valid`
        (bind _aswbp_cook_inventory (cast `/Game/Blueprints/UI/WBP_CookInventory` (`self.CurrentWidget`)))
        (`/Game/Blueprints/UI/WBP_CookInventory.UpdateInventory` _aswbp_cook_inventory (`|MakeArray` (`/Game/Blueprints/Cooking/Ingredients/BP_Ingredient.IngredientData` _selectedingredient)))
        (`self.K2_DestroyActor` (`self.SelectedIngredient`))
        (set `self.SelectedIngredient` null)))))

(fn `UserConstructionScript`)